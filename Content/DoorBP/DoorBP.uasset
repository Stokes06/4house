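; DoorBP is a sliding door actor that opens for the first-person character unless locked.
; Overlapping its trigger plays the DoorSlide timeline to move InnerDoorPiece along Z.
; Leaving plays a separate DoorReturn timeline in reverse from its end, so the piece snaps to that timeline's end position if interrupted mid-slide.
; Tick refreshes a LOCKED or UNLOCKED text label from IsDoorLocked, which also gates both movements.
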(event `self.ReceiveTick`
  (params (DeltaSeconds :type "Float (single-precision)"))
  (bind _lockedtext (`self.LockedText`))
  (if (`self.IsDoorLocked`)
    (`TextRenderComponent.K2_SetText` _lockedtext "LOCKED")
    (else
      (`TextRenderComponent.K2_SetText` _lockedtext "UNLOCKED"))))

(event `self.checkForPlayerTrigger.OnComponentBeginOverlap`
  (params (OverlappedComponent :type "PrimitiveComponent Object Reference") (OtherActor :type "Actor Object Reference") (OtherComp :type "PrimitiveComponent Object Reference") (OtherBodyIndex :type Integer) (bFromSweep :type Boolean) (SweepResult :type "HitResult Structure (by ref)"))
  (cast `/Game/FirstPersonBP/Blueprints/FirstPersonCharacter` OtherActor)
  (if (not (`self.IsDoorLocked`))
    (bind (_direction _slideamount) (`Timeline|DoorSlide` :!via `PlayFromStart`)
      (:`Update`
        (`SceneComponent.K2_SetRelativeLocation` (`self.InnerDoorPiece`) (`KismetMathLibrary.MakeVector` 0.0 0.0 (* _slideamount 50.0)) false false)))))

(event `self.checkForPlayerTrigger.OnComponentEndOverlap`
  (params (OverlappedComponent :type "PrimitiveComponent Object Reference") (OtherActor :type "Actor Object Reference") (OtherComp :type "PrimitiveComponent Object Reference") (OtherBodyIndex :type Integer))
  (cast `/Game/FirstPersonBP/Blueprints/FirstPersonCharacter` OtherActor)
  (if (not (`self.IsDoorLocked`))
    (bind (_direction _slideamount) (`Timeline|DoorReturn` :!via `ReverseFromEnd`)
      (:`Update`
        (`SceneComponent.K2_SetRelativeLocation` (`self.InnerDoorPiece`) (`KismetMathLibrary.MakeVector` 0.0 0.0 (* 50.0 _slideamount)) false false)))))

(fn `UserConstructionScript`)